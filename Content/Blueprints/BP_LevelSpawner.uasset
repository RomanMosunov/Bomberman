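; BP_LevelSpawner procedurally builds a randomized 2D grid level of walls, bricks and enemies at BeginPlay.
; Nested X/Z loops place cells relative to the actor, spaced by SpriteSize.
; Helper checks put walls on the border and at even-even interior cells, forming a pillar lattice.
; Open cells outside the clear starting-corner safe zone randomly receive a brick or, failing that, occasionally an enemy.
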(event `self.ReceiveBeginPlay`
  (bind (_returnvalue_x _returnvalue_y _returnvalue_z) (`KismetMathLibrary.BreakVector` (`self.K2_GetActorLocation`)))
  (bind _returnvalue_x_2 (`KismetMathLibrary.BreakVector` (`self.K2_GetActorLocation`)))
  (for _index (range (+ (`self.SizeX`) 1))
    (bind _output_get (set `self.IndexX` _index))
    (set `self.OffsetX` (`self.Offset` _output_get _returnvalue_x_2))
    (for _index_2 (range (+ (`self.SizeZ`) 1))
      (bind _output_get_2 (set `self.IndexZ` _index_2))
      (bind _result (`/Engine/EditorBlueprintResources/StandardMacros.NegateFloat` (`self.Offset` _output_get_2 _returnvalue_z))
        (:`  `
          (set `self.OffsetZ` _result)
          (if (`self.OuterWalls`)
            (`|SpawnActorFromClass` "/Game/Blueprints/BP_Wall.BP_Wall_C" (`KismetMathLibrary.MakeTransform` (`KismetMathLibrary.MakeVector` (`self.OffsetX`) 0.0 (`self.OffsetZ`))) "Undefined" "MultiplyWithRoot" null null)
            (elif (`self.InnerWalls`)
              (if (`self.SafeZone`)
                (if (`KismetMathLibrary.RandomBoolWithWeight` 0.5)
                  (`|SpawnActorFromClass` "/Game/Blueprints/BP_Brick.BP_Brick_C" (`KismetMathLibrary.MakeTransform` (`KismetMathLibrary.MakeVector` (`self.OffsetX`) 0.0 (`self.OffsetZ`))) "Undefined" "MultiplyWithRoot" null null)
                  (elif (`KismetMathLibrary.RandomBoolWithWeight` 0.1)
                    (`|SpawnActorFromClass` "/Game/Blueprints/BP_Enemy.BP_Enemy_C" (`KismetMathLibrary.MakeTransform` (`KismetMathLibrary.MakeVector` (`self.OffsetX`) 0.0 (`self.OffsetZ`))) "Undefined" "MultiplyWithRoot" null null))))
              (else
                (`|SpawnActorFromClass` "/Game/Blueprints/BP_Wall.BP_Wall_C" (`KismetMathLibrary.MakeTransform` (`KismetMathLibrary.MakeVector` (`self.OffsetX`) 0.0 (`self.OffsetZ`))) "Undefined" "MultiplyWithRoot" null null)))))))))

(fn `UserConstructionScript`)