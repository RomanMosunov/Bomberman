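; BP_Explosion is a grid-style, Paper2D flipbook explosion segment that damages overlapping actors and destroys itself when its animation finishes.
; Detonation spawns segments at the four direction components that are clear of BP_Wall, each starting a chain.
; ChainExplosion recursively spawns the next segment at its own Up transform with decremented Power, until Power runs out or a Wall-tagged overlap blocks it.
; The final zero-Power segment uses a different flipbook.
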(event `self.Sphere.OnComponentBeginOverlap`
  (params (OverlappedComponent :type "PrimitiveComponent Object Reference") (OtherActor :type "Actor Object Reference") (OtherComp :type "PrimitiveComponent Object Reference") (OtherBodyIndex :type Integer) (bFromSweep :type Boolean) (SweepResult :type "HitResult Structure (by ref)"))
  (`|ExecutionSequence`
    (:`then_0`
      (`GameplayStatics.ApplyDamage` OtherActor 1.0))
    (:`then_1`
      (if (`self.ActorHasTag` OtherActor "Wall")
        (set `self.CanSpawn` false)))))

(event `self.ReceiveBeginPlay`
  (`PaperFlipbookComponent.SetLooping` (`self.ExplosionSprite`) false))

(event `self.ExplosionSprite.OnFinishedPlaying`
  (`self.K2_DestroyActor`))

(event `Detonation`
  (for _array_element (`|MakeArray` (`self.Up`) (`self.Right`) (`self.Down`) (`self.Left`))
    (bind _ref2 (`self.CheckWalls` _array_element))
    (bind _returnvalue (`SceneComponent.K2_GetComponentToWorld` _ref2))
    (bind _returnvalue_2 (`|SpawnActorFromClass` "BP_Explosion_C" (`KismetMathLibrary.MakeTransform` (`KismetMathLibrary.MakeVector` (.x (.location _returnvalue)) (+ (.y (.location _returnvalue)) -0.1) (.z (.location _returnvalue))) (.rotation _returnvalue) (.scale _returnvalue)) "Undefined" "MultiplyWithRoot" null (`self.Power`) null))
    (`self.ChainExplosion` _returnvalue_2)))

(event `ChainExplosion`
  (bind _returnvalue (`SceneComponent.K2_GetComponentToWorld` (`self.Up`)))
  (`self.SetFlipBook`
    (:`Out`
      (bind _result (`self.CheckNewSpawn`)
        (:`  `
          (bind _returnvalue_2 (`|SpawnActorFromClass` "BP_Explosion_C" (`KismetMathLibrary.MakeTransform` (`KismetMathLibrary.MakeVector` (.x (.location _returnvalue)) (+ (.y (.location _returnvalue)) -0.1) (.z (.location _returnvalue))) (.rotation _returnvalue) (.scale _returnvalue)) "Undefined" "MultiplyWithRoot" null _result null))
          (`self.ChainExplosion` _returnvalue_2))))))

(fn `UserConstructionScript`)