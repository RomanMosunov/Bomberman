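; Player character for a Bomberman-style 2D game that moves on the XZ plane and plants bombs.
; Enhanced Input drives movement and switches directional walk or idle flipbooks based on the last facing.
; Bombs spawn snapped to a 16-unit grid with the player's BombPower, provided ammo remains and the player no longer overlaps the last one.
; Each plant starts a delayed loop that refills the bomb count to its maximum.
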(event `self.ReceiveBeginPlay`
  (set `self.BombsCount` (`self.BomdsMax`)))

(event `EnhancedInput|/Game/Input/IA_Move`
  (params (ActionValue :type "Vector2D Structure") (ElapsedSeconds :type "Float (double-precision)") (TriggeredSeconds :type "Float (double-precision)") (InputAction :type "InputAction Object Reference" :default "/Game/Input/IA_Move.IA_Move"))
  (:`Triggered`
    (`self.MovementInput` ActionValue)
    (`self.SwitchMoveAnim`))
  (:`Completed`
    (`self.SwitchIdleAnim`)))

(event `EnhancedInput|/Game/Input/IA_Bomb`
  (params (ActionValue :type Boolean) (ElapsedSeconds :type "Float (double-precision)") (TriggeredSeconds :type "Float (double-precision)") (InputAction :type "InputAction Object Reference" :default "/Game/Input/IA_Bomb.IA_Bomb"))
  (:`Triggered`
    (`self.CheckBombSpawnCondition`
      (:`Out`
        (`self.SpawnBomb`)
        (`self.Reload`)))))

(fn `MovementInput`
  (params (Value :type "Vector2D Structure"))
  (bind _output_get (set `self.MoveInput` Value))
  (bind (_returnvalue_x _returnvalue_y) (`KismetMathLibrary.BreakVector2D` (* _output_get (`self.MoveSpeed`))))
  (`self.AddMovementInput` (`KismetMathLibrary.MakeVector` _returnvalue_x 0.0 _returnvalue_y)))

(fn `SpawnBomb`
  (bind (_returnvalue_x _returnvalue_y _returnvalue_z) (`KismetMathLibrary.BreakVector` (`self.K2_GetActorLocation`)))
  (bind _returnvalue (`|SpawnActorFromClass` "/Game/Blueprints/BP_Bomb.BP_Bomb_C" (`KismetMathLibrary.MakeTransform` (`KismetMathLibrary.MakeVector` (`KismetMathLibrary.GridSnap_Float` _returnvalue_x 16.0) (+ _returnvalue_y -1.0) (`KismetMathLibrary.GridSnap_Float` _returnvalue_z 16.0))) "Undefined" "MultiplyWithRoot" null (`self.BombPower`) null))
  (set `self.LastPlantedBomb` _returnvalue)
  (`/Engine/EditorBlueprintResources/StandardMacros.DecrementInt` (`self.BombsCount`)))

(fn `UserConstructionScript`)